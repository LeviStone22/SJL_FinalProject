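; Melee troll enemy that takes sword, fire and frost hits and plays an attack montage through TrollAttack.
; Overlaps with player weapons or projectiles call ApplyDamage, based on the player's attack state.
; AnyDamage shows the health bar and, unless an animation is playing, plays a reaction, then subtracts health and reports to AI hearing/damage sense.
; Death there notifies the game mode and drops pickups; PointDamage has its own simpler death path.
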(event OnComponentBeginOverlap(CapsuleComponent)
  (params (OverlappedComponent :type Primitive%20Component%20Object%20Reference) (OtherActor :type Actor%20Object%20Reference) (OtherComp :type Primitive%20Component%20Object%20Reference) (OtherBodyIndex :type Integer) (bFromSweep :type Boolean) (SweepResult :type Hit%20Result%20Structure%20%28by%20ref%29))
  (Utilities|Casting|CastToWeapon_Sword OtherActor)
  (bind _asmelee_character (Utilities|Casting|CastToMelee_Character (Game|GetPlayerCharacter 0)))
  (Utilities|FlowControl|Sequence
    (:then_0
      (if (Variables|/Game/SamStuff/MeleeCharacter/Melee_Character.Melee_Character_C|GetSlashSword _asmelee_character)
        (if (Variables|Default|GetCanBeHitWithMelee)
          (Game|Damage|ApplyDamage self 0.25 0 0)
          (bind _returnvalue (Audio|SpawnSound2D "/Game/SamStuff/SwordSound/mixkit-sword-cutting-flesh-2788_Cue.mixkit-sword-cutting-flesh-2788_Cue" 0.8 1.0 0.0 0))
          (Utilities|FlowControl|DoOnce false) ; enters at Reset
        )))
    (:then_1
      (if (Variables|/Game/SamStuff/MeleeCharacter/Melee_Character.Melee_Character_C|GetSlashSword2 _asmelee_character)
        (if (Variables|Default|GetCanBeHitWithMelee)
          (Game|Damage|ApplyDamage self 0.5 0 0)
          (bind _returnvalue_2 (Audio|SpawnSound2D "/Game/SamStuff/SwordSound/mixkit-sword-cutting-flesh-2788_Cue.mixkit-sword-cutting-flesh-2788_Cue" 0.8 1.0 0.0 0))
          (Utilities|FlowControl|DoOnce false) ; enters at Reset
        )))))

(event Custom|TrollAttack
  (Animation|Montage|PlayMontage (Variables|Character|GetMesh) "/Game/InfinityBladeAdversaries/Enemy/Enemy_Troll/Enemy_Troll_Poison_Animation/AttackMontage_A.AttackMontage_A"))

(event Custom|VisibleHealth
  (Rendering|SetVisibility (Variables|Default|GetHealthBar) true false))

(event Collision|EventActorBeginOverlap
  (params (OtherActor :type Actor%20Object%20Reference))
  (bind _asmagic_character (Utilities|Casting|CastToMagicCharacter (Game|GetPlayerCharacter 0)))
  (Utilities|FlowControl|Sequence
    (:then_0
      (if (Variables|/Game/ThirdPersonBP/Blueprints/MagicCharacter.MagicCharacter_C|GetIsCastingFire _asmagic_character)
        (bind _asflame_projectile (Utilities|Casting|CastToFlameProjectile OtherActor))
        (Effects|SpawnEmitteratLocation "/Game/StarterContent/Particles/P_Explosion.P_Explosion" (Transformation|GetActorLocation _asflame_projectile))
        (Game|Damage|ApplyDamage self 0.5 0 0)
        (Actor|DestroyActor _asflame_projectile)))
    (:then_1
      (if (Variables|/Game/ThirdPersonBP/Blueprints/MagicCharacter.MagicCharacter_C|GetIsCastingIce _asmagic_character)
        (bind _asfrost_projectile (Utilities|Casting|CastToFrostProjectile OtherActor))
        (Effects|SpawnEmitteratLocation "/Game/InfinityBladeEffects/Effects/FX_Skill_Aura/P_Aura_Ice_Ending_01.P_Aura_Ice_Ending_01" (Transformation|GetActorLocation _asfrost_projectile))
        (Game|Damage|ApplyDamage self 0.25 0 0)
        (Actor|DestroyActor _asfrost_projectile)))))

(event Game|Damage|EventPointDamage
  (params (Damage :type Float%20%28single-precision%29) (DamageType :type Damage%20Type%20Object%20Reference) (HitLocation :type Vector :default "0, 0, 0") (HitNormal :type Vector :default "0, 0, 0") (HitComponent :type Primitive%20Component%20Object%20Reference) (BoneName :type Name :default "None") (ShotFromDirection :type Vector :default "0, 0, 0") (InstigatedBy :type Controller%20Object%20Reference) (DamageCauser :type Actor%20Object%20Reference) (HitInfo :type Hit%20Result%20Structure%20%28by%20ref%29))
  (Variables|Default|SetTrollHealth (- (Variables|Default|GetTrollHealth) Damage))
  (Class|AISenseDamage|ReportDamageEvent self DamageCauser Damage (.TraceStart (Collision|BreakHitResult HitInfo)))
  (Development|PrintString (Utilities|String|ToString(Float) Damage))
  (if (<= (Variables|Default|GetTrollHealth) 0.0)
    (Components|Animation|PlayAnimation (Variables|Character|GetMesh) "/Game/InfinityBladeAdversaries/Enemy/Enemy_Troll/Enemy_Troll_Poison_Animation/ExoGame_Troll_React_Death.ExoGame_Troll_React_Death" false)
    (Class|Pawn|DetachfromControllerPendingDestroy)
    (Collision|SetCollisionEnabled (Variables|Collision|GetCapsuleComponent) "NoCollision")
    (Utilities|FlowControl|Delay 3.33)
    (Actor|DestroyActor)))

(event Game|Damage|EventAnyDamage
  (params (Damage :type Float%20%28single-precision%29) (DamageType :type Damage%20Type%20Object%20Reference) (InstigatedBy :type Controller%20Object%20Reference) (DamageCauser :type Actor%20Object%20Reference))
  (CallFunction|VisibleHealth)
  (if (not (Audio|Components|Audio|IsPlaying (Variables|Character|GetMesh)))
    (Components|Animation|PlayAnimation (Variables|Character|GetMesh) "/Game/InfinityBladeAdversaries/Enemy/Enemy_Troll/Enemy_Troll_Poison_Animation/ExoGame_Troll_React_Heavy_Front.ExoGame_Troll_React_Heavy_Front" false)
    (Utilities|FlowControl|Delay 1.03)
    (Components|Animation|SetAnimationMode (Variables|Character|GetMesh) "AnimationBlueprint")
    (bind _output_get (Variables|Default|SetTrollHealth (- (Variables|Default|GetTrollHealth) Damage)))
    (Variables|/Game/SamStuff/AIStuff/AI_HealthWidget.AI_HealthWidget_C|SetHealthBar (Variables|Default|GetHealthWidgetRef) _output_get)
    (Class|AISenseDamage|ReportDamageEvent self (Game|GetPlayerCharacter 0) Damage (Transformation|GetActorLocation))
    (if (<= (Variables|Default|GetTrollHealth) 0.0)
      (bind _returnvalue (Audio|SpawnSound2D "/Game/JaneStuff/JaneSounds/trollDeath_Cue.trollDeath_Cue" 0.8 1.0 0.0 0))
      (Audio|Components|Audio|Play _returnvalue 0.0)
      (Components|Animation|PlayAnimation (Variables|Character|GetMesh) "/Game/InfinityBladeAdversaries/Enemy/Enemy_Troll/Enemy_Troll_Poison_Animation/ExoGame_Troll_React_Death.ExoGame_Troll_React_Death" false)
      (Class|Pawn|DetachfromControllerPendingDestroy)
      (Collision|SetCollisionEnabled (Variables|Collision|GetCapsuleComponent) "NoCollision")
      (Utilities|FlowControl|Delay 3.33)
      (Actor|DestroyActor)
      (bind _asthird_person_game_mode (Utilities|Casting|CastToThirdPersonGameMode (Game|GetGameMode)))
      (Default|EnemiesDefeatedDispEvent _asthird_person_game_mode)
      (Game|SpawnActorfromClass "/Game/ThirdPersonBP/Blueprints/HealthPickup.HealthPickup_C" (Math|Conversions|ToTransform(Vector) (Transformation|GetActorLocation)) "Undefined" 0 0)
      (Game|SpawnActorfromClass "/Game/ThirdPersonBP/Blueprints/MagickaPickup.MagickaPickup_C" (Math|Conversions|ToTransform(Vector) (Transformation|GetActorLocation)) "Undefined" 0 0)
      (else
        (Variables|Default|SetCanBeHitWithMelee false)
        (Utilities|FlowControl|Delay 1.0)
        (Variables|Default|SetCanBeHitWithMelee true)))))

(event EventBeginPlay
  (bind _asai_health_widget (Utilities|Casting|CastToAI_HealthWidget (UserInterface|GetUserWidgetObject (Variables|Default|GetHealthBar))))
  (Variables|Default|SetHealthWidgetRef _asai_health_widget))

(fn ConstructionScript)

(fn Death
  (Components|Animation|PlayAnimation (Variables|Character|GetMesh) "/Game/InfinityBladeAdversaries/Enemy/Enemy_Troll/Enemy_Troll_Poison_Animation/ExoGame_Troll_Death_.ExoGame_Troll_Death_" false)
  (Actor|DestroyActor))